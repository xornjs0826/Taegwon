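; BP_Helloactor is an actor that prints debug text and slides its Sphere component back and forth along relative X.
; BeginPlay prints the actor's name, increments X축의값, prints a counting loop and then "complete".
; Tick moves the Sphere by Speed scaled with delta time, flipping IsMoveX at fixed positive and negative limits to reverse direction.
; Disconnected nodes hold unused loop, print and sphere-rotation experiments.
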(event `self.ReceiveBeginPlay`
  ;[1 1 1] 코멘트
  (`KismetSystemLibrary.PrintString` (`KismetSystemLibrary.GetDisplayName` self) true true (struct :`G` 0.15599 :`B` 1.0 :`A` 1.0) 10.0)
  (set `self.x축의 값` (+ (`self.x축의 값`) 1.0))
  (for _index (range 101)
    (`KismetSystemLibrary.PrintString` (`KismetStringLibrary.Conv_IntToString` _index)))
  (`KismetSystemLibrary.PrintString` "complete" true true (struct :`G` 0.66 :`B` 1.0 :`A` 1.0) 60.0))

(event `self.ReceiveTick`
  (params (DeltaSeconds :type "Float (single-precision)"))
  (bind _sphere (`self.Sphere`))
  (bind _sphere_2 (`self.Sphere`))
  (bind _relativelocation_x (`KismetMathLibrary.BreakVector` (`SceneComponent.RelativeLocation` _sphere_2)))
  (bind _relativelocation_x_2 (`KismetMathLibrary.BreakVector` (`SceneComponent.RelativeLocation` _sphere)))
  ;[0.9012 0.8424 1 1 42] condition 값에 따라 True/False로 이벤트 실행
  (if (`self.isMove+X`)
    ;;[1 0.7855 0.2263 1 25] +X로 이동
    (`SceneComponent.K2_AddRelativeLocation` _sphere (`KismetMathLibrary.MakeVector` (* DeltaSeconds (`self.speed`))) false false)
    (if (>= _relativelocation_x_2 200.0)
      (set `self.isMove+X` false))
    (else
      ;;[0 0.2066 1 1 25] -x으로 이동
      (`SceneComponent.K2_AddRelativeLocation` _sphere_2 (`KismetMathLibrary.MakeVector` (* (* DeltaSeconds (`self.speed`)) -1.0)) false false)
      (if (<= _relativelocation_x -200.0)
        (set `self.isMove+X` true)))))

(fn `UserConstructionScript`)