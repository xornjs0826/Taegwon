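; BP_practice is a practice Blueprint that moves its Sphere component back and forth along its relative X axis.
; Each Tick offsets the Sphere by Speed scaled with DeltaSeconds, keeping the motion frame-rate independent.
; The TrueMove boolean picks the direction and flips when relative X reaches or passes either hard-coded bound, without clamping the overshoot.
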(event `self.ReceiveTick`
  (params (DeltaSeconds :type "Float (single-precision)"))
  (bind _sphere (`self.Sphere`))
  (bind _sphere_2 (`self.Sphere`))
  (bind _relativelocation_x (`KismetMathLibrary.BreakVector` (`SceneComponent.RelativeLocation` _sphere)))
  (bind _relativelocation_x_2 (`KismetMathLibrary.BreakVector` (`SceneComponent.RelativeLocation` _sphere_2)))
  (if (`self.true_move+`)
    (`SceneComponent.K2_AddRelativeLocation` _sphere_2 (`KismetMathLibrary.MakeVector` (* DeltaSeconds (`self.speed`))) false false)
    (if (>= _relativelocation_x_2 500.0)
      (set `self.true_move+` false))
    (else
      (`SceneComponent.K2_AddRelativeLocation` _sphere (`KismetMathLibrary.MakeVector` (* (* DeltaSeconds (`self.speed`)) -1.0)) false false)
      (if (<= _relativelocation_x 0.0)
        (set `self.true_move+` true)))))

(fn `UserConstructionScript`)